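; Actor for a melodic string of a rubab instrument that visibly vibrates and plays a note when struck.
; The Vibrate event restarts a timeline that drives Alpha and switches on the Fret name to play a sound for notes A to G.
; Tick jitters the string mesh by interpolating toward random offsets, blended from rest by Alpha.
; BeginPlay triggers one vibration with an empty fret after a short delay.
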(event Custom|Vibrate
  (params (Fret :type String))
  (bind _returnvalue (Transformation|GetActorLocation))
  (Utilities|FlowControl|Sequence
    (:then_0
      (bind _newtrack_0 (Timeline|Timeline PlayFromStart)
        (:Update
          (Variables|Default|SetAlpha _newtrack_0))))
    (:then_1
      (switch string Fret
        (:Note_D
          (Audio|PlaySoundatLocation 0 _returnvalue "0, 0, 0" 1.0 1.0 0.0 0 0 0 0))
        (:Note_E
          (Audio|PlaySoundatLocation 0 _returnvalue "0, 0, 0" 1.0 1.0 0.0 0 0 0 0))
        (:Note_F
          (Audio|PlaySoundatLocation 0 _returnvalue "0, 0, 0" 1.0 1.0 0.0 0 0 0 0))
        (:Note_G
          (Audio|PlaySoundatLocation 0 _returnvalue "0, 0, 0" 1.0 1.0 0.0 0 0 0 0))
        (:Note_A
          (Audio|PlaySoundatLocation 0 _returnvalue "0, 0, 0" 1.0 1.0 0.0 0 0 0 0))
        (:Note_B
          (Audio|PlaySoundatLocation 0 _returnvalue "0, 0, 0" 1.0 1.0 0.0 0 0 0 0))
        (:Note_C
          (Audio|PlaySoundatLocation 0 _returnvalue "0, 0, 0" 1.0 1.0 0.0 0 0 0 0))))))

(event EventBeginPlay
  (Utilities|FlowControl|Delay 1.0)
  (CallFunction|Vibrate))

(event EventTick
  (params (DeltaSeconds :type Float%20%28single-precision%29))
  (bind _sm_melodic_string_1 (Variables|Default|GetSM_Melodic_String_1))
  (Transformation|SetRelativeLocation _sm_melodic_string_1 (Math|Vector|Lerp(Vector) "0, 0, 0" (Math|Interpolation|VInterpTo (Variables|/Script/Engine.SceneComponent|GetRelativeLocation _sm_melodic_string_1) (Math|Vector|MakeVector (Math|Random|RandomFloatinRange -1.0 1.0) (Math|Random|RandomFloatinRange -1.0 1.0) (Math|Random|RandomFloatinRange -1.0 1.0)) (Utilities|Time|GetWorldDeltaSeconds) 5.0) (Variables|Default|GetAlpha)) false false))

(fn ConstructionScript)