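; BP_Rubab is the playable rubab for a VR music-learning experience, driven by a Socket.IO server.
; Incoming "note" events play mapped sounds, while "menu" events are passed to the VR pawn's Choice.
; For a chosen song, correct notes advance a hint dot and emissive string highlight through dynamic materials, ending in applause and a finish callback.
; In Level_PartsFunctions, a timed sequence moves highlight markers over the instrument's parts.
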(event OnConnected(SocketIOClient)
  (params (SocketId :type String) (SessionId :type String) (bIsReconnection :type Boolean))
  (bind _socketioclient (Variables|Default|GetSocketIOClient))
  (Development|PrintString "This works")
  (Class|SocketIOClientComponent|JoinNamespace _socketioclient)
  (Class|SocketIOClientComponent|BindEventtoDelegate _socketioclient "note" (delegate Custom|onNote) "/" "USE_DEFAULT")
  (Class|SocketIOClientComponent|BindEventtoDelegate _socketioclient "menu" (delegate Custom|onMenuInput) "/" "USE_DEFAULT"))

(event OnFail(SocketIOClient)
  (Development|PrintString "Failed"))

(event OnConnectionProblems(SocketIOClient)
  (params (Attempts :type Integer) (NextAttemptInMs :type Integer) (TimeSinceConnected :type Float%20%28single-precision%29))
  (Development|PrintString "Problem"))

(event OnSocketNamespaceConnected(SocketIOClient)
  (params (Namespace :type String))
  (Development|PrintString (Utilities|String|Append Namespace " Connected")))

(event OnSocketNamespaceDisconnected(SocketIOClient)
  (params (Namespace :type String))
  (Development|PrintString (Utilities|String|Append Namespace " Disconnected")))

(event OnGenericEvent(SocketIOClient)
  (params (EventName :type String) (EventData :type SIO%20Json%20Value%20Object%20Reference)))

(event Custom|onNote
  (params (EventData :type SIO%20Json%20Value%20Object%20Reference))
  (bind _returnvalue (Class|SIOJsonValue|AsString EventData))
  (bind _note_sound_map (Variables|Default|GetNote%20sound%20Map))
  (bind _translationmap (Variables|Default|GetTranslationMap))
  (bind _chosensongnotes (Variables|Default|GetChosenSongNotes))
  (bind _returnvalue_2 (Utilities|Array|LastIndex _chosensongnotes))
  (bind (_value _returnvalue_3) (Utilities|Map|Find _note_sound_map _returnvalue))
  (bind (_value_2 _returnvalue_4) (Utilities|Map|Find _translationmap _returnvalue))
  (Utilities|FlowControl|Sequence
    (:then_1
      ;[1 1 1] Play 2D sound of strings/frets played
      (Development|PrintString _returnvalue)
      (if _returnvalue_3
        (Audio|PlaySound2D _value 1.0 1.0 0.0 0 0)
        (else
          (Development|PrintString "cant find"))))
    (:then_2
      ;[1 1 1] Note visualization dot
      (if (Utilities|Array|IsNotEmpty (Variables|Default|GetChosenSongNotes))
        (if (Math|Boolean|ANDBoolean _returnvalue_4 (Utilities|Enum|Equal(Enum) _value_2 (Utilities|GetObjectName (Utilities|Array|Get(acopy) (Variables|Default|GetChosenSongNotes) (Variables|Default|GetVaryingID)))) (<= (Variables|Default|GetVaryingID) _returnvalue_2))
          (if (== (Variables|Default|GetVaryingID) (Utilities|Array|LastIndex (Variables|Default|GetChosenSongNotes)))
            (Development|SetHiddeninGame (Variables|Default|GetNoteHintViz) true false)
            (Audio|PlaySound2D "/Game/NarrativeMedia/NarrativeAudio/Applausekort.Applausekort" 1.0 1.0 0.0 0 0)
            (Variables|Default|SetVaryingID 0)
            (Default|CallOnFinishedPlaying)
            (else
              (CallFunction|UpdateNoteVisualisation (+ (Variables|Default|GetVaryingID) 1))
              (Variables|Default|SetVaryingID (+ (Variables|Default|GetVaryingID) 1))))
          (else
            (Development|PrintString (Utilities|String|Append (Utilities|String|ToString(Integer) (Variables|Default|GetVaryingID)) "/" (Utilities|String|ToString(Integer) _returnvalue_2)) true true "(R=0.914394,G=1.000000,B=0.000000,A=1.000000)")))))))

(event Custom|onMenuInput
  (params (EventData :type SIO%20Json%20Value%20Object%20Reference))
  (bind _returnvalue (Class|SIOJsonValue|AsString EventData))
  (Default|Choice (Variables|Default|GetReferenceVRPawn) _returnvalue)
  (Development|PrintString _returnvalue))

(event EventBeginPlay
  (bind _socketioclient (Variables|Default|GetSocketIOClient))
  ;[1 1 1] Song note order (composition)
  (Utilities|FlowControl|Sequence
    (:then_0
      (Variables|Default|SetSong1 (Utilities|Array|MakeArray (Variables|Default|GetS1_F1) (Variables|Default|GetS1_F3) (Variables|Default|GetS2_F00) (Variables|Default|GetS2_F1) (Variables|Default|GetS2_F3) (Variables|Default|GetS3_F00) (Variables|Default|GetS3_F2) (Variables|Default|GetS3_F3)))
      (Variables|Default|SetSong2 (Utilities|Array|MakeArray (Variables|Default|GetS2_F3) (Variables|Default|GetS3_F00) (Variables|Default|GetS3_F1) (Variables|Default|GetS3_F00) (Variables|Default|GetS3_F1) (Variables|Default|GetS3_F3) (Variables|Default|GetS2_F1) (Variables|Default|GetS2_F3) (Variables|Default|GetS3_F00) (Variables|Default|GetS2_F3) (Variables|Default|GetS3_F00) (Variables|Default|GetS2_F3) (Variables|Default|GetS1_F4) (Variables|Default|GetS2_F1) (Variables|Default|GetS2_F3) (Variables|Default|GetS2_F1) (Variables|Default|GetS2_F3) (Variables|Default|GetS2_F1) (Variables|Default|GetS1_F4) (Variables|Default|GetS1_F3) (Variables|Default|GetS1_F4) (Variables|Default|GetS2_F1) (Variables|Default|GetS1_F4) (Variables|Default|GetS1_F3) (Variables|Default|GetS2_F3)))
      (Variables|Default|SetSong3 (Utilities|Array|MakeArray (Variables|Default|GetS1_F4) (Variables|Default|GetS2_F1) (Variables|Default|GetS2_F3) (Variables|Default|GetS1_F4) (Variables|Default|GetS2_F3) (Variables|Default|GetS2_F4) (Variables|Default|GetS3_F1) (Variables|Default|GetS3_F1) (Variables|Default|GetS1_F1) (Variables|Default|GetS3_F1) (Variables|Default|GetS2_F4) (Variables|Default|GetS2_F3) (Variables|Default|GetS1_F4) (Variables|Default|GetS1_F4) (Variables|Default|GetS3_F1) (Variables|Default|GetS1_F4))))
    (:then_1
      (Class|SocketIOClientComponent|Connect _socketioclient (Utilities|String|Trim (Utilities|String|MakeLiteralString "http://172.19.65.69:3000")) "socket.io" "" 0 0)
      (Utilities|FlowControl|Delay 1.0)
      (Development|PrintString (Utilities|String|ToString(Boolean) (Variables|/Script/SocketIOClient.SocketIOClientComponent|GetbIsConnected _socketioclient)) true true "(R=1.000000,G=0.000000,B=0.894553,A=1.000000)" 2e+01))
    (:then_2
      (bind _returnvalue (Rendering|Material|CreateDynamicMaterialInstance (Variables|Default|GetS1_F0) 0 "/Game/Rubab/Materials/String_Materials/M_NylonString.M_NylonString" "None" :!class /Script/Engine.PrimitiveComponent))
      (Variables|Default|SetMaterial_highlightedstring1 _returnvalue)
      (bind _returnvalue_2 (Rendering|Material|CreateDynamicMaterialInstance (Variables|Default|GetS2_F0) 0 "/Game/Rubab/Materials/String_Materials/M_NylonString.M_NylonString" "None" :!class /Script/Engine.PrimitiveComponent))
      (Variables|Default|SetMaterial_highlightedstring2 _returnvalue_2)
      (bind _returnvalue_3 (Rendering|Material|CreateDynamicMaterialInstance (Variables|Default|GetS3_F0) 0 "/Game/Rubab/Materials/String_Materials/M_NylonString.M_NylonString" "None" :!class /Script/Engine.PrimitiveComponent))
      (Variables|Default|SetMaterial_highlightedstring3 _returnvalue_3))
    (:then_3
      ;[1 1 1] Highlighting parts movement
      (Rendering|SetVisibility (Variables|Default|GetHighlight) false false)
      (bind _returnvalue_4 (Game|GetCurrentLevelName true))
      (if (Utilities|Enum|Equal(Enum) _returnvalue_4 "Level_PartsFunctions")
        (Utilities|FlowControl|Delay 14.0)
        ;;[1 1 1] Goat skin is stretched over the lower part
        (Transformation|SetRelativeScale3D (Variables|Default|GetHighlight) "0.347757,0.241900,-0.007003")
        (Transformation|SetRelativeLocationAndRotation (Variables|Default|GetHighlight) "-24.894851,-11.168077,3.143331" "14.077126,3.688576,-234.187268" false false)
        (Rendering|SetVisibility (Variables|Default|GetHighlight) true false)
        ;;[1 1 1] Pegs
        (Utilities|FlowControl|Delay 16.0)
        (Transformation|SetRelativeScale3D (Variables|Default|GetHighlight) "0.292356,-0.123397,0.074537")
        (Transformation|SetRelativeLocationAndRotation (Variables|Default|GetHighlight) "17.357501,-8.395767,6.053335" "17.120384,5.993967,-233.567054" false false)
        (Rendering|SetVisibility (Variables|Default|GetHighlight1) true false)
        (Utilities|FlowControl|Delay 6.0)
        ;;[1 1 1] Main strings
        (Rendering|SetVisibility (Variables|Default|GetHighlight1) false false)
        (Transformation|SetRelativeScale3D (Variables|Default|GetHighlight) "0.963558,0.030497,0.034848")
        (Transformation|SetRelativeLocationAndRotation (Variables|Default|GetHighlight) "4.864013,-8.553738,12.000000" "14.725688,5.801063,-228.710500" false false)
        ;;[1 1 1] Sympathetic strings
        (Utilities|FlowControl|Delay 4.0)
        (Transformation|SetRelativeScale3D (Variables|Default|GetHighlight) "0.440707,0.073033,0.034848")
        (Transformation|SetRelativeLocationAndRotation (Variables|Default|GetHighlight) "-3.741398,-11.971521,6.679758" "11.595134,3.010011,-229.346318" false false)
        (Utilities|FlowControl|Delay 1e+01)
        (Rendering|SetVisibility (Variables|Default|GetHighlight) false false)))))

(event EventEndPlay
  (params (EndPlayReason :type EEndPlayReason%20Enum :default "Destroyed"))
  (Class|SocketIOClientComponent|Disconnect (Variables|Default|GetSocketIOClient)))

(event EventTick
  (params (DeltaSeconds :type Float%20%28single-precision%29))
  (Development|PrintString (Utilities|String|Append "Connected: " (Utilities|String|ToString(Boolean) (Variables|/Script/SocketIOClient.SocketIOClientComponent|GetbIsConnected (Variables|Default|GetSocketIOClient)))) true false "(R=0.000000,G=0.660000,B=1.000000,A=1.000000)" 2.0 "asdfw"))

(fn ConstructionScript)

(fn UpdateNoteVisualisation
  (params (Array%20ID :type Integer))
  (LocalVariables|SetSelectedSceneComp (Utilities|Array|Get(acopy) (Variables|Default|GetChosenSongNotes) Array%20ID))
  (Utilities|FlowControl|Sequence
    (:then_0
      (Rendering|Material|SetVectorParameterValue (Variables|Default|GetMaterial_highlightedstring1) "NylonParam" "(R=0.000000,G=0.000000,B=0.000000,A=0.000000)" :!class /Script/Engine.MaterialInstanceDynamic))
    (:then_1
      (bind _asstatic_mesh_component (Utilities|Casting|CastToStaticMeshComponent (LocalVariables|GetSelectedSceneComp))
        (:then
          (LocalVariables|SetStringMesh _asstatic_mesh_component))
        (:CastFailed
          (bind _asstatic_mesh_component_2 (Utilities|Casting|CastToStaticMeshComponent (Transformation|GetAttachParent (LocalVariables|GetSelectedSceneComp))))
          (LocalVariables|SetStringMesh _asstatic_mesh_component_2))))
    (:then_2
      (Transformation|SetWorldLocation (Variables|Default|GetNoteHintViz) (Transformation|GetWorldLocation (LocalVariables|GetSelectedSceneComp)) false false)
      (Development|SetHiddeninGame (Variables|Default|GetNoteHintViz) false false)
      (Development|PrintString (Utilities|String|ToString(Integer) Array%20ID) true true "(R=0.000000,G=0.660000,B=1.000000,A=1.000000)" 5e+01 "jiu")
      (if (Utilities|IsValid (LocalVariables|GetStringMesh))
        (bind _asmaterial_instance_dynamic (Utilities|Casting|CastToMaterialInstanceDynamic (Rendering|Material|GetMaterial (LocalVariables|GetStringMesh) 0)))
        (Rendering|Material|SetVectorParameterValue _asmaterial_instance_dynamic "NylonParam" "(R=1.000000,G=0.765068,B=0.005208,A=10.000000)" :!class /Script/Engine.MaterialInstanceDynamic) ; emissive color
      ))))

(fn DetermineSong
  (params (SongId :type Integer))
  (Variables|Default|SetChosenSongNotes (Utilities|Select :Index (- SongId 1) :Option%200 (Variables|Default|GetSong1) :Option%201 (Variables|Default|GetSong2) :Option%202 (Variables|Default|GetSong3)))
  (CallFunction|UpdateNoteVisualisation))

(fn ChangeStringColour
  (params (Snare1 :type Linear%20Color%20Structure :default "(R=0.947917,G=0.133301,B=0.133301,A=10.000000)") (Snare2 :type Linear%20Color%20Structure :default "(R=0.125678,G=0.588542,B=0.143935,A=10.000000)") (Snare3 :type Linear%20Color%20Structure :default "(R=0.161838,G=0.224977,B=0.817708,A=10.000000)"))
  (Rendering|Material|SetVectorParameterValue (Variables|Default|GetMaterial_highlightedstring1) "NylonParam" Snare1 :!class /Script/Engine.MaterialInstanceDynamic)
  (Rendering|Material|SetVectorParameterValue (Variables|Default|GetMaterial_highlightedstring2) "NylonParam" Snare2 :!class /Script/Engine.MaterialInstanceDynamic)
  (Rendering|Material|SetVectorParameterValue (Variables|Default|GetMaterial_highlightedstring3) "NylonParam" Snare3 :!class /Script/Engine.MaterialInstanceDynamic))